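; Hero_BP is the 2D flipbook player character, which jumps, scores for survival time and handles its own death.
; BeginPlay detaches the camera and starts a looping timer that feeds the score widget.
; Tick picks run, jump or dead flipbooks, and while dead creates a game-over widget with the score each frame.
; A DoOnce reset on landing limits jumping; PlayerDead adds another game-over widget, then pauses after a delay.
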(event `self.ReceiveTick`
  (params (DeltaSeconds :type "Float (single-precision)"))
  ;[1 1 1] animations
  (if (`self.isDead`)
    (`PaperFlipbookComponent.SetFlipbook` (`self.Sprite`) "/Game/character/_dead._dead")
    ;[1 1 1] player score
    (bind _returnvalue (`|CreateWidget` "/Game/BluePrints/GameOverBP.GameOverBP_C"))
    (bind _output_get (set `self.gameoverHUD` _returnvalue))
    (`TextBlock.SetText` (`/Game/BluePrints/GameOverBP.final` _output_get) (`KismetTextLibrary.Conv_IntToText` (`self.scoreInt`)))
    (`UserWidget.AddToViewport` _output_get 0)
    (elif (`NavMovementComponent.IsFalling` (`self.CharacterMovement`))
      (`PaperFlipbookComponent.SetFlipbook` (`self.Sprite`) "/Game/character/_jump._jump")
      (else
        (`PaperFlipbookComponent.SetFlipbook` (`self.Sprite`) "/Game/character/_run._run")))))

(event `self.ReceiveBeginPlay`
  (bind _returnvalue (`GameplayStatics.GetPlayerController` 0))
  ;[1 1 1] Events
  (set `PlayerController.bShowMouseCursor` false _returnvalue)
  (`WidgetBlueprintLibrary.SetInputMode_GameOnly` _returnvalue)
  (`SceneComponent.K2_DetachFromComponent` (`self.Camera`) "KeepWorld" "KeepWorld" "KeepWorld" true)
  (bind _returnvalue_2 (`|CreateWidget` "/Game/BluePrints/ScoreWidgetBP.ScoreWidgetBP_C"))
  (bind _output_get (set `self.score` _returnvalue_2))
  (`UserWidget.AddToViewport` _output_get 0)
  (`KismetSystemLibrary.K2_SetTimerDelegate` (delegate `updateScore`) 1.0 true))

(event `updateScore`
  ;[1 1 1] Events
  (if (not (`self.isDead`))
    (bind _result (`/Engine/EditorBlueprintResources/StandardMacros.IncrementInt` (`self.scoreInt`))
      (:`  `
        (`/Game/BluePrints/ScoreWidgetBP.updateScore` (`self.score`) _result)))))

(event `InputAction|Jump`
  (params (Key :type "Key Structure"))
  ;[1 1 1] Jumping
  (:`Pressed`
    (if (not (`self.isDead`))
      (`/Engine/EditorBlueprintResources/StandardMacros.DoOnce` false :!label _label
        (:`Completed`
          (`self.Jump`)
          (`GameplayStatics.PlaySound2D` "/Game/sfx/jump.jump" 0.5 1.0 0.0 null null))))))

(event `self.OnLanded`
  (params (Hit :type "HitResult Structure (by ref)"))
  ;[1 1 1] Jumping
  (goto _label :!via `Reset`))

(event `PlayerDead`
  ;[1 1 1] player death
  (set `self.isDead` true)
  (bind _returnvalue (`|CreateWidget` "/Game/BluePrints/GameOverBP.GameOverBP_C"))
  (`UserWidget.AddToViewport` _returnvalue 0)
  (`GameplayStatics.PlaySound2D` "/Game/sfx/death.death" 0.5 1.0 0.0 null null)
  (`KismetSystemLibrary.Delay` 0.3)
  (`GameplayStatics.SetGamePaused` true))

(fn `UserConstructionScript`)